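; Game mode for the main menu that shows the menu widget, plays audio and handles the fade-out transition.
; On BeginPlay it creates and caches the MainMenu widget, adds it to the viewport, then after a two-second delay starts the audio and shows the mouse cursor.
; ShowFadeOutUI lazily creates the UI_Fade_Out widget, fades out the audio and adds the overlay to the viewport.
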(event `self.ReceiveBeginPlay`
  (`/Engine/EditorBlueprintResources/StandardMacros.IsValid` (`self.MainMenu_Ref`)
    (:`Is Valid`
      _)
    (:`Is Not Valid`
      (bind _returnvalue (`|CreateWidget` "/Game/UserInterface/Main_Menu/MainMenu.MainMenu_C"))
      (bind _output_get (set `self.MainMenu_Ref` _returnvalue))))
  (`UserWidget.AddToViewport` _output_get 0)
  (`KismetSystemLibrary.Delay` 2.0)
  (`AudioComponent.Play` (`self.Audio`) 0.0)
  (set `PlayerController.bShowMouseCursor` true (`GameplayStatics.GetPlayerController` 0)))

(event `Show FadeOutUI`
  (`/Engine/EditorBlueprintResources/StandardMacros.IsValid` (`self.FadeOut_Ref`)
    (:`Is Valid`
      _)
    (:`Is Not Valid`
      (bind _returnvalue (`|CreateWidget` "/Game/UserInterface/Main_Menu/UI_Fade_Out.UI_Fade_Out_C"))
      (bind _output_get (set `self.FadeOut_Ref` _returnvalue))))
  (`AudioComponent.FadeOut` (`self.Audio`) 2.0 0.0 "Linear")
  (`KismetSystemLibrary.PrintString` "Hello")
  (`UserWidget.AddToViewport` _output_get 0))

(fn `UserConstructionScript`)