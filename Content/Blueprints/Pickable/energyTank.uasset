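; Energy tank pickup that restores a random amount of energy to the BP_CGRobo character.
; On overlap it adds the energy to the robot's Vita component, clamps it to the maximum, plays a pickup sound at its location and destroys itself.
; Tick spins the item mesh slowly around yaw at a frame-rate independent speed.
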(event `self.ReceiveTick`
  (params (DeltaSeconds :type "Float (single-precision)"))
  (`SceneComponent.K2_AddLocalRotation` (`self.Item`) (`KismetMathLibrary.MakeRotator` 0.0 0.0 (* DeltaSeconds 45.0)) false false))

(event `self.ReceiveActorBeginOverlap`
  (params (OtherActor :type "Actor Object Reference"))
  (bind _asbp_cgrobo (cast `/Game/Blueprints/BP_CGRobo` OtherActor))
  (bind _vita (`CGearsRobot.Vita` _asbp_cgrobo))
  (bind _output_get (set `HealthComponent.energia` (+ (`HealthComponent.energia` _vita) (`KismetMathLibrary.RandomFloatInRange` 10.0 20.0)) _vita))
  (bind _maxenergia (`HealthComponent.Maxenergia` _vita))
  (if (> _output_get _maxenergia)
    (set `HealthComponent.energia` _maxenergia _vita))
  (`GameplayStatics.SpawnSoundAtLocation` "/Engine/VREditor/Sounds/UI/Object_PickUp.Object_PickUp" (`self.K2_GetActorLocation`) (struct) 1.0 1.0 0.0 null null)
  (`self.K2_DestroyActor`))

(fn `UserConstructionScript`)