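; LifterKey is a spinning pickup that activates the elevator when one of the player robots touches it.
; Tick yaws the item mesh at a constant rate.
; On overlap with BP_CGRobo or BP_CGBucketRobot it sets ElevatorActive on GameInstance_CGears, shows the LifterKeyCollect widget, plays a pickup sound and destroys itself.
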(event `self.ReceiveTick`
  (params (DeltaSeconds :type "Float (single-precision)"))
  (`SceneComponent.K2_AddLocalRotation` (`self.Item`) (`KismetMathLibrary.MakeRotator` 0.0 0.0 (* DeltaSeconds 45.0)) false false))

(event `self.ReceiveActorBeginOverlap`
  (params (OtherActor :type "Actor Object Reference"))
  (cast `/Game/Blueprints/BP_CGRobo` OtherActor
    (:`then`
      _)
    (:`CastFailed`
      (cast `/Game/Blueprints/BP_CGBucketRobot` OtherActor)))
  (bind _asgame_instance_cgears (cast `GameInstance_CGears` (`GameplayStatics.GetGameInstance`)))
  (set `GameInstance_CGears.bElevatorActive` true _asgame_instance_cgears)
  (bind _returnvalue (`|CreateWidget` "/Game/UserInterface/LifterKeyCollect.LifterKeyCollect_C"))
  (`UserWidget.AddToViewport` _returnvalue 0)
  (`GameplayStatics.SpawnSoundAtLocation` "/Game/SoundDesign/PickUp_1.PickUp_1" (`self.K2_GetActorLocation`) (struct) 1.0 1.0 0.0 null null)
  (`self.K2_DestroyActor`))

(fn `UserConstructionScript`)