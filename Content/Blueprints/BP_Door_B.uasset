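; BP_Door_B is a double sliding door that opens and closes as the BP_CGRobo character passes through its trigger box.
; Begin and end overlap share one toggle on the Open flag, which plays a pressurized-door sound and runs a timeline forward or in reverse to slide both door meshes.
; A VerifyKey function checks the game instance's DoorsActive flag, but the overlap logic does not call it.
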(event `self.Box.OnComponentBeginOverlap`
  (params (OverlappedComponent :type "PrimitiveComponent Object Reference") (OtherActor :type "Actor Object Reference") (OtherComp :type "PrimitiveComponent Object Reference") (OtherBodyIndex :type Integer) (bFromSweep :type Boolean) (SweepResult :type "HitResult Structure (by ref)"))
  (bind _returnvalue (`self.K2_GetActorLocation`))
  (cast `/Game/Blueprints/BP_CGRobo` OtherActor)
  (if (`self.Open`) :!label _label
    (`GameplayStatics.PlaySoundAtLocation` "/Game/SoundDesign/ClosePressurizedDoor_Cue.ClosePressurizedDoor_Cue" _returnvalue (struct) 1.0 1.0 0.0 null null null)
    (set `self.Open` false)
    (bind (_direction _sliding_door_sx _sliding_door_dx) (`Timeline|Timeline_3` :!via `Reverse` :!label _label_2)
      (:`Update`
        (`|ExecutionSequence`
          (:`then_0`
            (`SceneComponent.K2_SetRelativeLocation` (`self.SM_Door1`) _sliding_door_sx false false))
          (:`then_1`
            (`SceneComponent.K2_SetRelativeLocation` (`self.SM_Door`) _sliding_door_dx false false)))))
    (else
      (`GameplayStatics.PlaySoundAtLocation` "/Game/SoundDesign/OpenPressurizedDoor_Cue.OpenPressurizedDoor_Cue" _returnvalue (struct) 1.0 1.0 0.0 null null null)
      (set `self.Open` true)
      (goto _label_2 :!via `PlayFromStart`))))

(event `self.Box.OnComponentEndOverlap`
  (params (OverlappedComponent :type "PrimitiveComponent Object Reference") (OtherActor :type "Actor Object Reference") (OtherComp :type "PrimitiveComponent Object Reference") (OtherBodyIndex :type Integer))
  (cast `/Game/Blueprints/BP_CGRobo` OtherActor)
  (goto _label))

(fn `UserConstructionScript`)